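; BPC_Item3 is a child item Blueprint that can be cashed out to add its value to the player's cash.
; Its CashOut event calls CheckOverlapIsCashOutSpotNDestroy on the other actor, then passes Value to CashOutValuetoPlayerCash.
; The CashOutValuetoPlayerCash override and construction script only call their parent versions, and the BeginPlay, overlap and Tick events are disabled stubs.
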(event `self.CashOut`
  (params (OtherActor :type "Actor Object Reference"))
  ;[1 1 1] Custom Event and Functions from Parent
  (`self.CheckOverlapIsCashOutSpotNDestroy` OtherActor)
  (`self.CashOutValuetoPlayerCash` (`self.Value`)))

(fn `CashOutValuetoPlayerCash`
  (params (CashValue :type "Float (double-precision)"))
  (`parent.CashOutValuetoPlayerCash` CashValue))

(fn `UserConstructionScript`
  (`parent.UserConstructionScript`))