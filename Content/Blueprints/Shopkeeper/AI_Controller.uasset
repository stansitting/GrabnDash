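; AI controller for the shopkeeper that runs the BT_AIShopkeeper behavior tree on BeginPlay.
; AI Perception updates write the perceived actor to TargetActor and set the SeenPlayer? flag on the Blackboard.
; When sensing fails, it clears the flag and stores the stimulus location as LastSeenLocation.
; A forgotten target also clears the flag.
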(event `self.ReceiveBeginPlay`
  (`self.RunBehaviorTree` "/Game/Blueprints/Shopkeeper/BT_AIShopkeeper.BT_AIShopkeeper"))

(event `self.AIPerception.OnTargetPerceptionUpdated`
  (params (Actor :type "Actor Object Reference") (Stimulus :type "AIStimulus Structure"))
  (bind _blackboard (`self.Blackboard`))
  (`BlackboardComponent.SetValueAsObject` (`self.Blackboard`) "TargetActor" Actor)
  (if Stimulus_bSuccessfullySensed
    (`BlackboardComponent.SetValueAsBool` _blackboard "SeenPlayer?" true)
    (else
      (`BlackboardComponent.SetValueAsBool` _blackboard "SeenPlayer?" false)
      (`BlackboardComponent.SetValueAsVector` _blackboard "LastSeenLocation" Stimulus_StimulusLocation))))

(event `self.AIPerception.OnTargetPerceptionForgotten`
  (params (Actor :type "Actor Object Reference"))
  (`BlackboardComponent.SetValueAsBool` (`self.Blackboard`) "SeenPlayer?" false))

(fn `UserConstructionScript`)